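; Boss enemy that creeps toward the player while firing rapid bullets with random pitch spread, and destroys the player on overlap with a death effect.
; On BeginPlay it spawns a ring of shield minions attached to OrbitPivot, which spins every tick around the pitch axis.
; Minion death notifications decrement a counter that drops the shield at zero.
; Damage only reduces boss health while unshielded, destroying it when health runs out.
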(event `NotifyMinionDestroyed`
  (bind _output_get (set `self.ActiveMinions` (- (`self.ActiveMinions`) 1)))
  (if (<= _output_get 0)
    (set `self.IsShielded` false)))

(event `self.ReceiveBeginPlay`
  (bind _returnvalue (`GameplayStatics.GetActorOfClass` "/Game/BP_Player.BP_Player_C"))
  (set `self.Target` _returnvalue)
  (for _index (range 6)
    (bind _returnvalue_2 (`|SpawnActorFromClass` "/Game/BP_ShieldMinion.BP_ShieldMinion_C" (`self.GetTransform`) "Undefined" "MultiplyWithRoot" null null))
    (`self.K2_AttachToComponent` _returnvalue_2 (`self.OrbitPivot`) "None" "KeepRelative" "KeepRelative" "KeepRelative" true)
    (`self.K2_SetActorRelativeLocation` _returnvalue_2 (* (`KismetMathLibrary.GetForwardVector` (`KismetMathLibrary.MakeRotator` 0.0 (`KismetMathLibrary.Conv_IntToDouble` (* _index 60)))) 200.0) false false)
    (set `self.ActiveMinions` (+ (`self.ActiveMinions`) 1))))

(event `self.ReceiveTick`
  (params (DeltaSeconds :type "Float (single-precision)"))
  (`SceneComponent.K2_AddLocalRotation` (`self.OrbitPivot`) (`KismetMathLibrary.MakeRotator` 0.0 (* DeltaSeconds 90.0)) false false)
  (`/Engine/EditorBlueprintResources/StandardMacros.IsValid` (`self.Target`)
    (:`Is Valid`
      (`|ExecutionSequence`
        (:`then_0`
          (bind _output_get (set `self.Timer` (+ (`self.Timer`) DeltaSeconds)))
          (if (> _output_get 0.15)
            (set `self.Timer` 0.0)
            (`|SpawnActorFromClass` "/Game/BP_Bullet.BP_Bullet_C" (`KismetMathLibrary.MakeTransform` (.location (`SceneComponent.K2_GetComponentToWorld` (`self.FirePos`))) (`KismetMathLibrary.MakeRotator` (.roll (.rotation (`SceneComponent.K2_GetComponentToWorld` (`self.FirePos`)))) (+ (.pitch (.rotation (`SceneComponent.K2_GetComponentToWorld` (`self.FirePos`)))) (`KismetMathLibrary.RandomFloatInRange` -90.0 90.0)) (.yaw (.rotation (`SceneComponent.K2_GetComponentToWorld` (`self.FirePos`))))) (.scale (`SceneComponent.K2_GetComponentToWorld` (`self.FirePos`)))) "Undefined" "MultiplyWithRoot" null true 20.0 null)))
        (:`then_1`
          (`self.K2_AddActorWorldOffset` (* (`KismetMathLibrary.Normal` (- (`self.K2_GetActorLocation` (`self.Target`)) (`self.K2_GetActorLocation`))) 0.5)))))))

(event `self.ReceiveAnyDamage`
  (params (Damage :type "Float (single-precision)") (DamageType :type "DamageType Object Reference") (InstigatedBy :type "Controller Object Reference") (DamageCauser :type "Actor Object Reference"))
  (if (not (`self.IsShielded`))
    (bind _output_get (set `self.BossHp` (- (`self.BossHp`) Damage)))
    (if (<= _output_get 0.0)
      (`self.K2_DestroyActor`))))

(event `self.ReceiveActorBeginOverlap`
  (params (OtherActor :type "Actor Object Reference"))
  (bind _asbp_player (cast `/Game/BP_Player` OtherActor))
  (`NiagaraFunctionLibrary.SpawnSystemAtLocation` "/Game/NS_PlayerDeath.NS_PlayerDeath" (`self.K2_GetActorLocation` _asbp_player))
  (`self.K2_DestroyActor` _asbp_player))

(fn `UserConstructionScript`)