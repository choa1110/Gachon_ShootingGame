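; BP_EnemySpawner is an actor that repeatedly spawns a random entry from its SpawnPool at its own transform.
; BeginPlay waits an initial delay, then enables actor tick.
; Tick accumulates a timer, and once it passes the next spawn time, Spawn resets it, picks a new interval with random jitter around SpawnInterval, and spawns the actor.
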(event `self.ReceiveBeginPlay`
  (`KismetSystemLibrary.Delay` (`self.InitialDelay`))
  (`self.SetActorTickEnabled` true))

(event `self.ReceiveTick`
  (params (DeltaSeconds :type "Float (single-precision)"))
  (bind _output_get (set `self.Timer` (+ (`self.Timer`) DeltaSeconds)))
  (if (> _output_get (`self.NextSpawnTime`))
    (`self.Spawn`)))

(fn `Spawn`
  (bind _randomoffsetrange (`self.RandomOffsetRange`))
  (set `self.NextSpawnTime` (+ (`self.SpawnInterval`) (`KismetMathLibrary.RandomFloatInRange` (* _randomoffsetrange -1.0) _randomoffsetrange)))
  (set `self.Timer` 0.0)
  (`|SpawnActorFromClass` (`KismetArrayLibrary.Array_Random` (`self.SpawnPool`)) (`self.GetTransform`) "Undefined" "MultiplyWithRoot" null null))

(fn `UserConstructionScript`)