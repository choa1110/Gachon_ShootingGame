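; BP_Bullet is a projectile actor used by both the player and enemies, with an IsEnemy flag setting which side it hurts.
; Each tick it moves along its local X axis by Speed, without delta-time scaling.
; On overlap it ignores other bullets; enemy bullets hit only BP_Player, while others hit any non-player actor.
; A hit spawns the NS_Death effect, applies fixed damage and destroys the bullet.
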(event `self.ReceiveTick`
  (params (DeltaSeconds :type "Float (single-precision)"))
  (`self.K2_AddActorLocalOffset` (`KismetMathLibrary.MakeVector` (`self.Speed`))))

(event `self.ReceiveActorBeginOverlap`
  (params (OtherActor :type "Actor Object Reference"))
  (bind _isenemy (`self.isEnemy`))
  (cast `/Game/BP_Bullet` OtherActor
    (:`CastFailed`
      (cast `/Game/BP_Player` OtherActor
        (:`then`
          (if _isenemy
            (`NiagaraFunctionLibrary.SpawnSystemAtLocation` "/Game/NS_Death.NS_Death" (`self.K2_GetActorLocation`) :!label _label)
            (`GameplayStatics.ApplyDamage` OtherActor 10.0)
            (`self.K2_DestroyActor`)))
        (:`CastFailed`
          (if (not _isenemy)
            (goto _label)))))))

(fn `UserConstructionScript`)